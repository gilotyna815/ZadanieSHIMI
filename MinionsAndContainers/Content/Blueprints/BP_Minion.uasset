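; Minion AI pawn that takes an order for a gem type and walks to the nearest container that needs it.
; On spawn it stores its number and caches all BP_Container actors, since none are added at runtime.
; When interacted with, it filters containers by needed gem, picks the closest, moves there with AI Move To and prints status messages.
; Its interact sphere notifies the first-person character on entering and leaving range.
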(event `OnSpawned`
  (params (MinionNumber :type Integer))
  ;[1 1 1] Spawned
  (set `self.minionNumber` MinionNumber)
  ;;[1 1 1] Cannot be added during runtime so can be cached on spawn
  (bind _outactors (`GameplayStatics.GetAllActorsOfClass` "/Game/Blueprints/BP_Container.BP_Container_C"))
  (set `self.allContainers` _outactors)
  (`KismetSystemLibrary.PrintString` (`KismetStringLibrary.Concat_StrStr` "Spawned " (`self.GetMinionName`) ".")))

(event `self.InteractSphere.OnComponentBeginOverlap`
  (params (OverlappedComponent :type "PrimitiveComponent Object Reference") (OtherActor :type "Actor Object Reference") (OtherComp :type "PrimitiveComponent Object Reference") (OtherBodyIndex :type Integer) (bFromSweep :type Boolean) (SweepResult :type "HitResult Structure (by ref)"))
  ;[1 1 1] Player enters interact sphere
  (bind _asbp_first_person_character (cast `/Game/Blueprints/BP_FirstPersonCharacter` OtherActor))
  (`/Game/Blueprints/BP_FirstPersonCharacter.OnEnteredInteractRange` _asbp_first_person_character))

(event `self.InteractSphere.OnComponentEndOverlap`
  (params (OverlappedComponent :type "PrimitiveComponent Object Reference") (OtherActor :type "Actor Object Reference") (OtherComp :type "PrimitiveComponent Object Reference") (OtherBodyIndex :type Integer))
  ;[1 1 1] Player enters interact sphere
  (bind _asbp_first_person_character (cast `/Game/Blueprints/BP_FirstPersonCharacter` OtherActor))
  (`/Game/Blueprints/BP_FirstPersonCharacter.OnLeftInteractRange` _asbp_first_person_character))

(event `OnInteracted`
  (params (ChosenObject :type "/Game/Blueprints/ENeededObject Enum" :default "NewEnumerator0"))
  (bind _returnvalue (select `/Game/Blueprints/ENeededObject` (`self.Chosen Object`) :`NewEnumerator0` "a Ruby." :`NewEnumerator1` "an Emerald." :`NewEnumerator2` "a Sapphire." :`NewEnumerator3` "a Tourmaline." :`NewEnumerator4` "a Citrine." :`NewEnumerator5` "a Zircon." :`NewEnumerator6` "a Diamond."))
  ;[1 1 1] Interacted
  (set `self.Chosen Object` ChosenObject)
  ;;[1 1 1] Reset helper variables
  (`KismetArrayLibrary.Array_Clear` (`self.validContainers`))
  (set `self.shortestDistanceToValidContainer` 0.0)
  (set `self.nearestValidContainer` null)
  ;;[1 1 1] Are there any containers?
  (if (> (`KismetArrayLibrary.Array_Length` (`self.allContainers`)) 0)
    ;;[1 1 1] Choose valid containers (those that need the chosen object)
    (for _array_element (`self.allContainers`)
      (if (== (`/Game/Blueprints/BP_Container.NeededObject` _array_element) (`self.Chosen Object`))
        (`KismetArrayLibrary.Array_Add` (`self.validContainers`) _array_element)))
    ;;[1 1 1] Are there any valid containers?
    (if (> (`KismetArrayLibrary.Array_Length` (`self.validContainers`)) 0)
      ;;[1 1 1] Choose nearest valid container
      (for _array_element_2 (`self.validContainers`)
        ;;;[1 1 1] The distance cannot be zero
        (if (> (`self.shortestDistanceToValidContainer`) 0.0)
          (bind _returnvalue_2 (`KismetMathLibrary.Vector_Distance` (`SceneComponent.K2_GetComponentLocation` (`/Game/Blueprints/BP_Container.DefaultSceneRoot` _array_element_2)) (`SceneComponent.K2_GetComponentLocation` (`self.CapsuleComponent`))))
          ;;;[1 1 1] Found nearer container
          (if (< _returnvalue_2 (`self.shortestDistanceToValidContainer`))
            (set `self.shortestDistanceToValidContainer` _returnvalue_2 :!label _label)
            (set `self.nearestValidContainer` _array_element_2))
          (else
            (goto _label))))
      (`KismetSystemLibrary.PrintString` (`KismetStringLibrary.Concat_StrStr` (`self.GetMinionName`) " has found the nearest Container for " (select `/Game/Blueprints/ENeededObject` (`self.Chosen Object`) :`NewEnumerator0` "rubies" :`NewEnumerator1` "emeralds" :`NewEnumerator2` "sapphires" :`NewEnumerator3` "tourmalines" :`NewEnumerator4` "citrines" :`NewEnumerator5` "zircons" :`NewEnumerator6` "diamonds") " and is now travelling towards it with " _returnvalue))
      ;;[1 1 1] Move to the chosen container
      (`|AIMoveTo` self (0.0 0.0 0.0) (`self.nearestValidContainer`)
        (:`OnSuccess`
          ;;;[1 1 1] Reached the container
          (`KismetSystemLibrary.PrintString` (`KismetStringLibrary.Concat_StrStr` (`self.GetMinionName`) ": The " (`|GetEnumeratorNameAsString` (`self.Chosen Object`)) " has been delivered to the nearest Container for it.")))
        (:`OnFail`
          ;;;[1 1 1] Couldn't reach the container
          (`KismetSystemLibrary.PrintString` (`KismetStringLibrary.Concat_StrStr` (`self.GetMinionName`) ": The nearest Container for " (select `/Game/Blueprints/ENeededObject` (`self.Chosen Object`) :`NewEnumerator0` "rubies" :`NewEnumerator1` "emeralds" :`NewEnumerator2` "sapphires" :`NewEnumerator3` "tourmalines" :`NewEnumerator4` "citrines" :`NewEnumerator5` "zircons" :`NewEnumerator6` "diamonds") " could not have been reached."))))
      (`KismetSystemLibrary.PrintString` (`KismetStringLibrary.Concat_StrStr` (`self.GetMinionName`) " is awaiting further orders."))
      (else
        ;;[1 1 1] No containers to chose from
        (`KismetSystemLibrary.PrintString` (`KismetStringLibrary.Concat_StrStr` (`self.GetMinionName`) ": No Container is designated for " _returnvalue) :!label _label_2)))
    (else
      (goto _label_2))))

(fn `GetMinionName`
  (returns (MinionName :type String))
  (return (`KismetStringLibrary.BuildString_Int` "Minion " "#" (`self.minionNumber`))))

(fn `UserConstructionScript`)